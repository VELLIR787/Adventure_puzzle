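; BedroomBack is a clickable actor that switches the player's view to a fixed bedroom camera, apparently as a back-navigation control.
; Clicking its Widget component plays a door sound and adds a BlackScreen widget to the viewport.
; It then spawns a new orthographic CameraActor at a hardcoded transform on each click and makes it player 0's view target.
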(event OnClicked(Widget)
  (params (TouchedComponent :type Primitive%20Component%20Object%20Reference) (ButtonPressed :type Key%20Structure :default "None"))
  ;[1 1 1] Spawn Bedroom camera
  (Audio|PlaySound2D "/Game/Sound/DoorSound.DoorSound" 1.0 1.0 0.0 0 0)
  (bind _returnvalue (UserInterface|CreateWidget "/Game/UI/BlackScreen.BlackScreen_C"))
  (UserInterface|Viewport|AddtoViewport _returnvalue 0)
  (bind _returnvalue_2 (Game|SpawnActorfromClass "/Script/Engine.CameraActor" (Math|Transform|MakeTransform "-658.000000,-1762.000000,464.000000" "-21.000000,120.000000,0.000000") "Undefined" "MultiplyWithRoot" 0 0))
  (Class|CameraComponent|SetProjectionMode (Variables|/Script/Engine.CameraActor|GetCameraComponent _returnvalue_2) "Orthographic")
  (Class|CameraComponent|SetOrthoWidth (Variables|/Script/Engine.CameraActor|GetCameraComponent _returnvalue_2) 1795.0)
  (Class|CameraComponent|SetOrthoFarClipPlane (Variables|/Script/Engine.CameraActor|GetCameraComponent _returnvalue_2) 2952272.5)
  (Game|Player|SetViewTargetwithBlend (Game|GetPlayerController 0) _returnvalue_2 0.0 "VTBlend_Linear" 0.0 false))

(fn ConstructionScript)