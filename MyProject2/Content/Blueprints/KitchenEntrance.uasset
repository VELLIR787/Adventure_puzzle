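; KitchenEntrance is a Blueprint for a point-and-click kitchen entrance, gated behind a clickable key pickup.
; Clicking the Cube destroys it, reveals the Widget component and shows a FoundKey UI.
; Clicking the Widget component adds a BlackScreen overlay, then spawns an orthographic CameraActor at a hard-coded transform and switches the player's view target to it.
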(event OnClicked(Widget)
  (params (TouchedComponent :type Primitive%20Component%20Object%20Reference) (ButtonPressed :type Key%20Structure :default "None"))
  (bind _returnvalue (UserInterface|CreateWidget "/Game/UI/BlackScreen.BlackScreen_C"))
  (UserInterface|Viewport|AddtoViewport _returnvalue 0)
  (bind _returnvalue_2 (Game|SpawnActorfromClass "/Script/Engine.CameraActor" (Math|Transform|MakeTransform "-6820.000000,-1930.000000,690.000000" "-28.000000,50.000000,0.000000") "Undefined" "MultiplyWithRoot" 0 0))
  (Class|CameraComponent|SetProjectionMode (Variables|/Script/Engine.CameraActor|GetCameraComponent _returnvalue_2) "Orthographic")
  (Class|CameraComponent|SetOrthoWidth (Variables|/Script/Engine.CameraActor|GetCameraComponent _returnvalue_2) 1795.0)
  (Class|CameraComponent|SetOrthoFarClipPlane (Variables|/Script/Engine.CameraActor|GetCameraComponent _returnvalue_2) 2952272.5)
  (Game|Player|SetViewTargetwithBlend (Game|GetPlayerController 0) _returnvalue_2 0.0 "VTBlend_Linear" 0.0 false))

(event OnClicked(Cube)
  (params (TouchedComponent :type Primitive%20Component%20Object%20Reference) (ButtonPressed :type Key%20Structure :default "None"))
  (Components|DestroyComponent TouchedComponent)
  (Rendering|SetVisibility (Variables|Default|GetWidget) true false)
  (bind _returnvalue (UserInterface|CreateWidget "/Game/UI/FoundKey.FoundKey_C"))
  (UserInterface|Viewport|AddtoViewport _returnvalue 0))

(event EventBeginPlay)

(event Collision|EventActorBeginOverlap
  (params (OtherActor :type Actor%20Object%20Reference)))

(event EventTick
  (params (DeltaSeconds :type Float%20%28single-precision%29)))

(fn ConstructionScript)